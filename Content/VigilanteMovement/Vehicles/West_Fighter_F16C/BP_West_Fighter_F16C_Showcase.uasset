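; Static showcase variant of the West F-16C fighter that demonstrates the asset's functionality through UI sliders, checkboxes and buttons.
; Input events forward values to vehicle functions for flight controls, throttle, landing gear, canopy, air brake, lights, damage mode and afterburner.
; Buttons switch the gun's Niagara effect on and off.
; BeginPlay runs the parent logic, then turns off lights and sets a starting exhaust nozzle position.
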(event `self.ReceiveBeginPlay`
  ;[1 1 1] Static Showcase Demonstration of Asset functionality. Connects Inputs as Sliders, Buttons and Checkboxes to vehicle functions
  (`parent.ReceiveBeginPlay`)
  (`self.TurnOffLights`)
  (`self.SetExhaustNozzles` 0.6))

(event `/Game/VigilanteMovement/Shared/Blueprints/HUD/Showcase/Interfaces/BP_ShowcaseControlsInterface.SetSliderVariable0`
  (params (NewValue :type "Float (double-precision)"))
  ;[1 1 1] Static Showcase Demonstration of Asset functionality. Connects Inputs as Sliders, Buttons and Checkboxes to vehicle functions
  (`self.SetYaw` NewValue))

(event `/Game/VigilanteMovement/Shared/Blueprints/HUD/Showcase/Interfaces/BP_ShowcaseControlsInterface.SetSliderVariable1`
  (params (NewValue :type "Float (double-precision)"))
  ;[1 1 1] Static Showcase Demonstration of Asset functionality. Connects Inputs as Sliders, Buttons and Checkboxes to vehicle functions
  (`self.SetLightsIntensity` NewValue))

(event `/Game/VigilanteMovement/Shared/Blueprints/HUD/Showcase/Interfaces/BP_ShowcaseControlsInterface.SetSliderVariable2`
  (params (NewValue :type "Float (double-precision)"))
  ;[1 1 1] Static Showcase Demonstration of Asset functionality. Connects Inputs as Sliders, Buttons and Checkboxes to vehicle functions
  (set `self.Throttle` NewValue)
  (`self.SetThrottle`))

(event `/Game/VigilanteMovement/Shared/Blueprints/HUD/Showcase/Interfaces/BP_ShowcaseControlsInterface.SetTwinSliderVariable0`
  (params (`bFirstSlider?` :type Boolean) (NewFirstValue :type "Float (double-precision)") (NewSecondValue :type "Float (double-precision)"))
  ;[1 1 1] Static Showcase Demonstration of Asset functionality. Connects Inputs as Sliders, Buttons and Checkboxes to vehicle functions
  (`self.RetractFrontWheel` NewFirstValue)
  (`self.RetractRearLWheel` NewSecondValue)
  (`self.RetractRearRWheel` NewSecondValue))

(event `/Game/VigilanteMovement/Shared/Blueprints/HUD/Showcase/Interfaces/BP_ShowcaseControlsInterface.SetTwinSliderVariable1`
  (params (`bFirstSlider?` :type Boolean) (NewFirstValue :type "Float (double-precision)") (NewSecondValue :type "Float (double-precision)"))
  ;[1 1 1] Static Showcase Demonstration of Asset functionality. Connects Inputs as Sliders, Buttons and Checkboxes to vehicle functions
  (`self.SetCanopy` NewFirstValue)
  (`self.SetAirBrake` NewSecondValue))

(event `/Game/VigilanteMovement/Shared/Blueprints/HUD/Showcase/Interfaces/BP_ShowcaseControlsInterface.SetTwinSliderVariable2`
  (params (`bFirstSlider?` :type Boolean) (NewFirstValue :type "Float (double-precision)") (NewSecondValue :type "Float (double-precision)"))
  ;[1 1 1] Static Showcase Demonstration of Asset functionality. Connects Inputs as Sliders, Buttons and Checkboxes to vehicle functions
  (`self.SetPitch` NewFirstValue)
  (`self.SetRoll` NewSecondValue))

(event `/Game/VigilanteMovement/Shared/Blueprints/HUD/Showcase/Interfaces/BP_ShowcaseControlsInterface.SetCheckboxVariable0`
  (params (NewState :type Boolean))
  ;[1 1 1] Static Showcase Demonstration of Asset functionality. Connects Inputs as Sliders, Buttons and Checkboxes to vehicle functions
  (`self.SetDamagedMode` NewState))

(event `/Game/VigilanteMovement/Shared/Blueprints/HUD/Showcase/Interfaces/BP_ShowcaseControlsInterface.SetCheckboxVariable1`
  (params (NewState :type Boolean))
  ;[1 1 1] Static Showcase Demonstration of Asset functionality. Connects Inputs as Sliders, Buttons and Checkboxes to vehicle functions
  (`self.ToggleAfterburner` NewState))

(event `/Game/VigilanteMovement/Shared/Blueprints/HUD/Showcase/Interfaces/BP_ShowcaseControlsInterface.SetButtonsVariable0`
  (params (NewIndex :type Integer))
  ;[1 1 1] Static Showcase Demonstration of Asset functionality. Connects Inputs as Sliders, Buttons and Checkboxes to vehicle functions
  (switch `int` NewIndex
    (:`0`
      (`ActorComponent.SetActive` (`self.NS_Gun`) true false))
    (:`1`
      (`ActorComponent.SetActive` (`self.NS_Gun`) false false))))

(fn `UserConstructionScript`
  (`parent.UserConstructionScript`))