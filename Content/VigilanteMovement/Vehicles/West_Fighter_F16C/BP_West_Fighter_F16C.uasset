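; Child Blueprint for the F-16C fighter that turns flight control values into aircraft animation and VFX.
; Events map pitch, roll, yaw, throttle, gear, airbrake and canopy values onto its AnimBP, moving control surfaces, cockpit controls and parts.
; Throttle and afterburner state set exhaust nozzle size, which also drives Niagara jet scale and opacity.
; Gun VFX toggles only while the weapon system's active weapon is the Gun.
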(event `self.ReceiveBeginPlay`
  (`parent.ReceiveBeginPlay`)
  ;[1 1 1] Sets ABP Instances References
  (bind _asbpa_west_fighter_f16c (cast `/Game/VigilanteMovement/Vehicles/West_Fighter_F16C/BPA_West_Fighter_F16C` (`SkeletalMeshComponent.GetAnimInstance` (`self.SkeletalMesh`))))
  (set `self.AnimInstance` _asbpa_west_fighter_f16c)
  ;[1 1 1] Initial Exhaust and afterburner Settings
  (`self.SetExhaustNozzles` 0.6)
  (`NiagaraComponent.SetVariableVec3` (`self.NS_Jet`) "JetScale" (0.5 0.2 0.2))
  (`NiagaraComponent.SetVariableVec3` (`self.NS_Jet`) "JetRingsScale" (10.0 10.0 11.0))
  (`FXSystemComponent.SetFloatParameter` (`self.NS_Jet`) "Opacity divide" 0.8)
  (`self.SetAfterburner`))

(event `self.SetGear`
  (params (Value :type "Float (double-precision)"))
  ;[1 1 1] Sets Landing Gear Position
  (`self.RetractFrontWheel` Value)
  (`self.RetractRearLWheel` Value)
  (`self.RetractRearRWheel` Value))

(event `RetractFrontWheel`
  (params (Value :type "Float (double-precision)"))
  ;[1 1 1] Sets Front Gear Position
  (set `/Game/VigilanteMovement/Vehicles/West_Fighter_F16C/BPA_West_Fighter_F16C.FrontWheelRetract` Value (`self.AnimInstance`)))

(event `RetractRearLWheel`
  (params (Value :type "Float (double-precision)"))
  ;[1 1 1] Sets Rear Gears Position
  (set `/Game/VigilanteMovement/Vehicles/West_Fighter_F16C/BPA_West_Fighter_F16C.RearWheelLRetract` Value (`self.AnimInstance`)))

(event `RetractRearRWheel`
  (params (Value :type "Float (double-precision)"))
  ;[1 1 1] Sets Rear Gears Position
  (set `/Game/VigilanteMovement/Vehicles/West_Fighter_F16C/BPA_West_Fighter_F16C.RearWheelRRetract` Value (`self.AnimInstance`)))

(event `self.SetYaw`
  (params (Value :type "Float (double-precision)"))
  (bind _returnvalue (* Value -1.0))
  ;[1 1 1] Sets Yaw on Rudders and Pilot Pedals
  (set `/Game/VigilanteMovement/Vehicles/West_Fighter_F16C/BPA_West_Fighter_F16C.RuddersAngle` (`KismetMathLibrary.MapRangeClamped` _returnvalue -1.0 1.0 -45.0 45.0) (`self.AnimInstance`))
  (bind _output_get (set `/Game/VigilanteMovement/Vehicles/West_Fighter_F16C/BPA_West_Fighter_F16C.PedalLAngle` (* (`KismetMathLibrary.MapRangeClamped` _returnvalue -1.0 1.0 -10.0 10.0) -1.0) (`self.AnimInstance`)))
  (set `/Game/VigilanteMovement/Vehicles/West_Fighter_F16C/BPA_West_Fighter_F16C.PedalRAngle` _output_get (`self.AnimInstance`)))

(event `self.SetRoll`
  (params (Value :type "Float (double-precision)"))
  (bind _returnvalue (* Value -1.0))
  ;[1 1 1] Set Roll on Ailerons and Pilot Stick
  (bind _output_get (set `/Game/VigilanteMovement/Vehicles/West_Fighter_F16C/BPA_West_Fighter_F16C.FlapsOuterLAngle` (`KismetMathLibrary.MapRangeClamped` _returnvalue -1.0 1.0 -60.0 60.0) (`self.AnimInstance`)))
  (set `/Game/VigilanteMovement/Vehicles/West_Fighter_F16C/BPA_West_Fighter_F16C.FlapsOuterRAngle` (* _output_get -1.0) (`self.AnimInstance`))
  (set `/Game/VigilanteMovement/Vehicles/West_Fighter_F16C/BPA_West_Fighter_F16C.CenterStickRoll` (`KismetMathLibrary.MapRangeClamped` (* _returnvalue -1.0) -1.0 1.0 -25.0 25.0) (`self.AnimInstance`)))

(event `self.SetPitch`
  (params (Pitch :type "Float (double-precision)"))
  ;[1 1 1] Sets Pitch on Stabilizers and Pilot Stick
  (bind _output_get (set `/Game/VigilanteMovement/Vehicles/West_Fighter_F16C/BPA_West_Fighter_F16C.StabilizerLAngle` (`KismetMathLibrary.MapRangeClamped` (* Pitch -1.0) -1.0 1.0 -30.0 30.0) (`self.AnimInstance`)))
  (set `/Game/VigilanteMovement/Vehicles/West_Fighter_F16C/BPA_West_Fighter_F16C.StabilizerRAngle` _output_get (`self.AnimInstance`))
  (set `/Game/VigilanteMovement/Vehicles/West_Fighter_F16C/BPA_West_Fighter_F16C.CenterStickPitch` (`KismetMathLibrary.MapRangeClamped` Pitch -1.0 1.0 -25.0 25.0) (`self.AnimInstance`)))

(event `self.SetThrottle`
  ;[1 1 1] Sets Throttle on Exhausts and Pilot Left Hand Lever
  (set `/Game/VigilanteMovement/Vehicles/West_Fighter_F16C/BPA_West_Fighter_F16C.ThrottlePosition` (`KismetMathLibrary.MapRangeClamped` (`self.Throttle`) 0.0 1.0 -5.0 5.0) (`self.AnimInstance`))
  (if (not (`self.isAfterburnerActive`))
    (`self.SetExhaustNozzles` (`KismetMathLibrary.MapRangeClamped` (`self.Throttle`) 0.0 1.0 1.0 0.6))))

(event `SetExhaustNozzles`
  (params (Value :type "Float (double-precision)"))
  ;[1 1 1] Sets Exhaust Nozzles Size
  (bind _output_get (set `/Game/VigilanteMovement/Vehicles/West_Fighter_F16C/BPA_West_Fighter_F16C.ExhaustNozzles` Value (`self.AnimInstance`)))
  (bind _returnvalue (`KismetMathLibrary.MapRangeClamped` _output_get 0.0 1.0 0.115 0.17))
  (`NiagaraComponent.SetVariableVec3` (`self.NS_Jet`) "JetScale" (`KismetMathLibrary.MakeVector` (`KismetMathLibrary.MapRangeClamped` _output_get 0.0 1.0 0.25 0.9) _returnvalue _returnvalue))
  (`NiagaraComponent.SetVariableVec3` (`self.NS_Jet`) "JetRingsScale" (`KismetMathLibrary.MakeVector` 10.0 10.0 (`KismetMathLibrary.MapRangeClamped` _output_get 0.0 1.0 6.0 12.0)))
  (`FXSystemComponent.SetFloatParameter` (`self.NS_Jet`) "Opacity divide" (`KismetMathLibrary.MapRangeClamped` _output_get 0.0 1.0 10.0 1.0)))

(event `self.SetAirBrake`
  (params (Value :type "Float (double-precision)"))
  ;[1 1 1] Sets AirBrake Position
  (set `/Game/VigilanteMovement/Vehicles/West_Fighter_F16C/BPA_West_Fighter_F16C.Airbrake` (`KismetMathLibrary.MapRangeClamped` Value 0.0 1.0 0.0 1.0) (`self.AnimInstance`)))

(event `self.SetCanopy`
  (params (Value :type "Float (double-precision)"))
  ;[1 1 1] Sets Canopy Position
  (set `/Game/VigilanteMovement/Vehicles/West_Fighter_F16C/BPA_West_Fighter_F16C.Canopy` (`KismetMathLibrary.MapRangeClamped` Value 0.0 1.0 0.0 35.0) (`self.AnimInstance`)))

(event `self.SetAfterburner`
  (bind _isafterburneractive (`self.isAfterburnerActive`))
  ;[1 1 1] Activates Afterburner VFX and Exhaust size
  (`ActorComponent.SetActive` (`self.NS_Jet`) _isafterburneractive true)
  (if _isafterburneractive
    (`self.SetExhaustNozzles` 1.0)
    (else
      (`self.SetExhaustNozzles` 0.6))))

(event `self.StarGunVFX`
  ;[1 1 1] Activates and Deactivates Gun VFX
  (if (== (`/Game/VigilanteMovement/Shared/Blueprints/Weapon/BP_WeaponComponent.Get Active Weapon Name` (`self.WeaponSystem`)) "Gun")
    (`ActorComponent.SetActive` (`self.NS_Gun`) true false)))

(event `self.StopGunVFX`
  ;[1 1 1] Activates and Deactivates Gun VFX
  (if (== (`/Game/VigilanteMovement/Shared/Blueprints/Weapon/BP_WeaponComponent.Get Active Weapon Name` (`self.WeaponSystem`)) "Gun")
    (`ActorComponent.SetActive` (`self.NS_Gun`) false false)))

(fn `UserConstructionScript`
  (`parent.UserConstructionScript`))