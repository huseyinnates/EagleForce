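; BP_UAV is a UAV actor that climbs vertically in a Cesium georeferenced world.
; On BeginPlay it adds a Cesium globe anchor component and stores its longitude, latitude and height in Position.
; Each Tick grows PositionIncrement with delta time and adds the whole total to the actor's world Z, so the climb keeps accelerating.
; Position is then refreshed from the anchor after every move.
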(event `self.ReceiveBeginPlay`
  (bind _returnvalue (`AddComponent|NODE_AddCesiumGlobeAnchorComponent-0`))
  (bind _output_get (set `self.as` _returnvalue))
  (set `self.Position` (`CesiumGlobeAnchorComponent.GetLongitudeLatitudeHeight` _output_get)))

(event `self.ReceiveTick`
  (params (DeltaSeconds :type "Float (single-precision)"))
  (bind (_returnvalue_x _returnvalue_y _returnvalue_z) (`KismetMathLibrary.BreakVector` (`self.K2_GetActorLocation`)))
  (bind _output_get (set `self.PositionIncrement` (+ (* DeltaSeconds 4.0) (`self.PositionIncrement`))))
  (`self.K2_SetActorLocation` (`KismetMathLibrary.MakeVector` _returnvalue_x _returnvalue_y (+ _returnvalue_z _output_get)))
  (set `self.Position` (`CesiumGlobeAnchorComponent.GetLongitudeLatitudeHeight` (`self.as`))))

(fn `UserConstructionScript`)