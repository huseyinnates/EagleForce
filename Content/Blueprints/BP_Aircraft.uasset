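; BP_Aircraft is an actor that flies along the spline of a referenced UAVPTrack.
; MoveAircraft plays the UAVMOVER timeline at a rate set by Duration, starting from UAVStartOffset.
; Each update maps the timeline alpha to spline distance and applies that world transform, so rotation follows the path.
; Pressing B starts the movement, and releasing it prints a debug message.
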(event `MoveAircraft`
  (bind _uavmover (`self.UAVMOVER`))
  (`TimelineComponent.SetPlayRate` _uavmover (/ 1.0 (`self.Duration`)))
  (`TimelineComponent.SetNewTime` _uavmover (`self.UAVStartOffset`))
  (bind (_direction _alpha) (`Timeline|UAVMOVER`)
    (:`Update`
      (set `self.Alpha` _alpha)
      (`self.K2_SetActorTransform` (`SplineComponent.GetTransformAtDistanceAlongSpline` (`UAVPathTrack.SplineTrack` (`self.UAVPTrack`)) (`KismetMathLibrary.Lerp` 0.0 (`SplineComponent.GetSplineLength` (`UAVPathTrack.SplineTrack` (`self.UAVPTrack`))) (`self.Alpha`)) "World" false)))))

(event `Key|B`
  (params (Key :type "Key Structure"))
  (:`Pressed`
    (`self.MoveAircraft`))
  (:`Released`
    (`KismetSystemLibrary.PrintString` "Should Work!")))

(fn `UserConstructionScript`)