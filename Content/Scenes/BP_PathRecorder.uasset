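; BP_PathRecorder is an actor that records its Cesium globe position as a row in a path table.
; On BeginPlay it adds a CesiumGlobeAnchor component, prints its longitude, latitude and height, and starts a timeline.
; When the timeline finishes, it passes the current coordinates to PathTrackCreator's AddRowToTable, saving a single point.
; Pressing A nudges the actor by a fixed horizontal offset.
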(event `self.ReceiveBeginPlay`
  (bind (_returnvalue_x _returnvalue_y _returnvalue_z) (`KismetMathLibrary.BreakVector` (`CesiumGlobeAnchorComponent.GetLongitudeLatitudeHeight` (`self.CesiumGlobeAnchor`))))
  (bind _returnvalue (`AddComponent|NODE_AddCesiumGlobeAnchorComponent-0`))
  (bind _output_get (set `self.CesiumGlobeAnchor` _returnvalue))
  (`KismetSystemLibrary.PrintString` (`KismetStringLibrary.Conv_VectorToString` (`CesiumGlobeAnchorComponent.GetLongitudeLatitudeHeight` _output_get)))
  (`KismetSystemLibrary.PrintString` (`KismetStringLibrary.Conv_VectorToString` (`CesiumGlobeAnchorComponent.GetLongitudeLatitudeHeight` (`self.CesiumGlobeAnchor`))))
  (`Timeline|Timeline`
    (:`Finished`
      (`PathTrackCreator.AddRowToTable` (`self.PathTrackCreator`) _returnvalue_x _returnvalue_y _returnvalue_z)
      (`KismetSystemLibrary.PrintString` "Data saved successfully!"))))

(event `self.ReceiveTick`
  (params (DeltaSeconds :type "Float (single-precision)")))

(event `Key|A`
  (params (Key :type "Key Structure"))
  (bind (_returnvalue_x _returnvalue_y _returnvalue_z) (`KismetMathLibrary.BreakVector` (`self.K2_GetActorLocation`)))
  (:`Pressed`
    (`self.K2_SetActorLocation` (`KismetMathLibrary.MakeVector` (+ _returnvalue_x 4.0) (+ _returnvalue_y 3.0) _returnvalue_z))))

(fn `UserConstructionScript`)